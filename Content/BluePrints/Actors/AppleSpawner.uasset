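; Apple spawner actor that drops an Apple at a random point along a local Y-axis span and hands it to a DiglettActor.
; BeginPlay caches the first Diglett found; SpawnApple, not triggered within this graph, waits a delay before spawning unless StopSpawning has disabled it.
; A grounded callback assigned to each apple tells Diglett to grab the latest one.
; The construction script locks EndPoint to Y with a minimum length.
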(event Custom|SpawnApple
  (if (Variables|Default|GetcanSpawn)
    (Utilities|FlowControl|Delay (Variables|Default|GetspawnDelay))
    (bind _returnvalue (Game|SpawnActorfromClass "/Game/BluePrints/Actors/Apple.Apple_C" (Math|Transform|MakeTransform (+ (Math|Vector|MakeVector 0.0 (* (.Y (Math|Vector|BreakVector (Variables|Default|GetEndPoint))) (Math|Random|RandomFloat)) 0.0) (Transformation|GetActorLocation))) "Undefined" 0 self 0))
    (EventDispatchers|AssignAppleIsGrounded _returnvalue (delegate Custom|AppleIsGroundIt))))

(event Custom|AppleIsGroundIt
  (bind _diglett (Variables|Default|GetDiglett))
  (Utilities|IsValid _diglett
    (:Is%20Valid
      (Default|GrabApple _diglett (stale Custom|SpawnApple _returnvalue)))))

(event EventBeginPlay
  (bind _outactors (Actor|GetAllActorsOfClass "/Game/BluePrints/character/DiglettActor.DiglettActor_C"))
  (if (> (Utilities|Array|Length _outactors) 0)
    (Variables|Default|SetDiglett (Utilities|Array|Get(acopy) _outactors))))

(fn ConstructionScript
  (if (< (.Y (Math|Vector|BreakVector (Variables|Default|GetEndPoint))) 1e+02)
    (Variables|Default|SetEndPoint "0,100.000000, 0")
    (else
      (Variables|Default|SetEndPoint (Math|Vector|MakeVector 0.0 (.Y (Math|Vector|BreakVector (Variables|Default|GetEndPoint))) 0.0)))))

(fn StopSpawning
  (Variables|Default|SetcanSpawn false))