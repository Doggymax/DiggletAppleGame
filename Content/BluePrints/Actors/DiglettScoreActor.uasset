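; DiglettScoreActor is an animated Diglett prop that digs along Z while spinning, with its own sound.
; On BeginPlay it starts the audio, then runs the DiglettDig timeline after StartDelay.
; The timeline's Completion track scales HowDeep and Rotation into the Digglet component's relative height and yaw.
; Inverted actors first snap to the full depth and rotation, then play the timeline in reverse.
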(event Custom|SetUnderGroundPosition
  (bind _digglet (Variables|Default|GetDigglet))
  (bind _returnvalue (Transformation|GetRelativeTransform _digglet))
  (if (Variables|Default|Getinverted)
    (Transformation|SetRelativeTransform _digglet (Math|Transform|MakeTransform (Math|Vector|MakeVector (.x (.location _returnvalue)) (.y (.location _returnvalue)) (Variables|Default|GethowDeep)) (Math|Rotator|MakeRotator (.roll (.rotation _returnvalue)) (.pitch (.rotation _returnvalue)) (Variables|Default|Getrotation)) (.scale _returnvalue)) false false)))

(event EventBeginPlay
  (bind _digglet (Variables|Default|GetDigglet))
  (bind _returnvalue (Transformation|GetRelativeTransform _digglet))
  (bind _returnvalue_2 (AddComponent|AddAudioComponent false))
  (bind _output_get (Variables|Default|SetAudioComponnent _returnvalue_2))
  (Audio|Components|Audio|SetSound _output_get (Variables|Default|Getaudio))
  (Audio|Components|Audio|Play _output_get 0.0)
  (CallFunction|SetUnderGroundPosition)
  (Utilities|FlowControl|Delay (Variables|Default|GetstartDelay))
  (if (Variables|Default|Getinverted)
    (bind _completion (Timeline|DiglettDig ReverseFromEnd)
      (:Update
        (Transformation|SetRelativeTransform _digglet (Math|Transform|MakeTransform (Math|Vector|MakeVector (.x (.location _returnvalue)) (.y (.location _returnvalue)) (* (Variables|Default|GethowDeep) _completion)) (Math|Rotator|MakeRotator (.roll (.rotation _returnvalue)) (.pitch (.rotation _returnvalue)) (* (Variables|Default|Getrotation) _completion)) (.scale _returnvalue)) false false)))
    (else
      (Timeline|DiglettDig PlayFromStart))))

(event Collision|EventActorBeginOverlap
  (params (OtherActor :type Actor%20Object%20Reference)))

(event EventTick
  (params (DeltaSeconds :type Float%20%28single-precision%29)))

(fn ConstructionScript)