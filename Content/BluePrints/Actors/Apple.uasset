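; Collectible apple actor that the Pikachu character picks up in an apple-collection game mode.
; Overlap on component S with PikachuBP adds a player apple through AppleCollectGM and destroys the actor.
; On destruction, it asks its Spawner, if valid, to spawn another apple.
; From BeginPlay, a delayed loop polls the apple's location until it stops changing, then sets IsGrounded and calls AppleIsGrounded.
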(event OnComponentBeginOverlap(s)
  (params (OverlappedComponent :type Primitive%20Component%20Object%20Reference) (OtherActor :type Actor%20Object%20Reference) (OtherComp :type Primitive%20Component%20Object%20Reference) (OtherBodyIndex :type Integer) (bFromSweep :type Boolean) (SweepResult :type Hit%20Result%20Structure%20%28by%20ref%29))
  (Utilities|Casting|CastToPikachuBP OtherActor)
  (bind _asapple_collect_gm (Utilities|Casting|CastToAppleCollectGM (Game|GetGameMode)))
  (Default|AddPlayerApple _asapple_collect_gm)
  (Actor|DestroyActor))

(event Custom|OnAppleDestroyed
  (params (DestroyedActor :type Actor%20Object%20Reference))
  (bind _spawner (Variables|Default|Getspawner))
  (Utilities|IsValid _spawner
    (:Is%20Valid
      (Default|SpawnApple _spawner))))

(event Custom|StartGrounCheck
  (bind _apple (Variables|Default|Getapple))
  (bind _returnvalue (Transformation|GetWorldLocation _apple))
  (Variables|Default|SetlastLocation (Transformation|GetWorldLocation (Variables|Default|Getapple)))
  (Utilities|FlowControl|Delay (Variables|Default|GetcheckDelay) :!label _label)
  (if (Math|Vector|Equal(Vector) (Variables|Default|GetlastLocation) _returnvalue 0.01)
    (Variables|Default|SetisGrounded true)
    (Default|CallAppleIsGrounded)
    (else
      (Variables|Default|SetlastLocation _returnvalue)
      (goto _label))))

(event EventBeginPlay
  (EventDispatchers|AssignOnDestroyed (delegate Custom|OnAppleDestroyed))
  (CallFunction|StartGrounCheck))

(event Collision|EventActorBeginOverlap
  (params (OtherActor :type Actor%20Object%20Reference)))

(event EventTick
  (params (DeltaSeconds :type Float%20%28single-precision%29)))

(fn ConstructionScript)