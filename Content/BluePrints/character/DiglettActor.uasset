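; Diglett actor that pops up at an apple's spot to grab it for the apple collecting game.
; GrabApple moves it under the apple, attaches the apple to AppleHolder, calls GoUp, then GoDown after a delay.
; The MoveUp timeline, reversed for descent, drives the heights of Diglett, holder and ground.
; When it finishes un-reversed, it destroys the apple and credits Diglett through AppleCollectGM.
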(event Custom|Go%20Up
  (bind _apple (Variables|Default|Getapple))
  (Variables|Default|SetgoingDown false)
  (bind _goupfloat (Timeline|MoveUp Play)
    (:Update
      (Variables|Default|SethowHi _goupfloat)
      (CallFunction|UpdateDiglett))
    (:Finished
      (if (not (Variables|Default|GetgoingDown))
        (Utilities|IsValid _apple
          (:Is%20Valid
            (Actor|DestroyActor _apple)
            (bind _asapple_collect_gm (Utilities|Casting|CastToAppleCollectGM (Game|GetGameMode)))
            (Default|AddDiglettApple _asapple_collect_gm)))))))

(event Custom|Go%20Down
  (bind _apple (Variables|Default|Getapple))
  (Variables|Default|SetgoingDown true)
  (bind _goupfloat (Timeline|MoveUp Reverse)
    (:Update
      (Variables|Default|SethowHi _goupfloat)
      (CallFunction|UpdateDiglett))
    (:Finished
      (if (not (Variables|Default|GetgoingDown))
        (Utilities|IsValid _apple
          (:Is%20Valid
            (Actor|DestroyActor _apple)
            (bind _asapple_collect_gm (Utilities|Casting|CastToAppleCollectGM (Game|GetGameMode)))
            (Default|AddDiglettApple _asapple_collect_gm)))))))

(event Custom|UpdateDiglett
  (Transformation|SetRelativeLocation (Variables|Default|Getdiglett) (Math|Vector|MakeVector 0.0 0.0 (* (Variables|Default|GethowHi) (Variables|Default|GetdeepDigglet))) false false)
  (Transformation|SetRelativeLocation (Variables|Default|GetAppleHolder) (Math|Vector|MakeVector 0.0 0.0 (+ (* (Variables|Default|GethowHi) (Variables|Default|GetdeepDigglet)) 8.0)) true false)
  (Transformation|SetRelativeLocation (Variables|Default|Getground) (Math|Vector|MakeVector 0.0 0.0 (* (Variables|Default|GethowHi) (Variables|Default|GetdeepGround))) false false))

(event Custom|GrabApple
  (params (apple :type Apple%20Object%20Reference))
  (bind _returnvalue (Transformation|GetActorTransform))
  (bind _returnvalue_2 (Transformation|GetActorTransform apple))
  (bind (_location _rotation _scale) (Math|Transform|BreakTransform _returnvalue))
  (bind (_x _y) (Math|Vector|BreakVector (.location _returnvalue_2)))
  (Variables|Default|Setapple apple)
  (Transformation|SetActorTransform (Math|Transform|MakeTransform (Math|Vector|MakeVector _x _y 0.0) _rotation _scale))
  (Transformation|AttachComponentToComponent (Variables|/Script/Engine.Actor|GetRootComponent apple) (Variables|Default|GetAppleHolder) "None" "SnapToTarget" "SnapToTarget" "KeepRelative" true)
  (CallFunction|GoUp)
  (Utilities|FlowControl|Delay (Variables|Default|GetdeleayBeforGround))
  (CallFunction|GoDown))

(fn ConstructionScript)