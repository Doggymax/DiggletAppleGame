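; Game mode for a timed apple-collecting match between the player and Diglett.
; BeginPlay creates the in-game widget, finds the AppleSpawner and starts music at the game instance's volume.
; StartPlaying begins spawning and runs a timeline countdown, which on finish stops spawning, notifies the widget and fades the music.
; GameFinished sends both apple tallies to the game instance and opens the winner's level; a tie opens none.
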(event Custom|Add%20player%20apple
  ;[1 1 1] Add Apples
  (Variables|Default|SetyourApples (+ (Variables|Default|GetyourApples) 1)))

(event Custom|Add%20Diglett%20Apple
  ;[1 1 1] Add Apples
  (Variables|Default|SetdiglettsApplels (+ (Variables|Default|GetdiglettsApplels) 1)))

(event Custom|Start%20Playing
  (Default|SpawnApple (Variables|Default|GetAppleSpawner))
  (bind _timeleft (Timeline|GameTime Play)
    (:Update
      (Variables|Default|SetsecLeft (Math|Float|Truncate _timeleft)))
    (:Finished
      (Default|StopSpawning (Variables|Default|GetAppleSpawner))
      (Default|TimerOut (Variables|Default|GetInGameWidget))
      (Audio|Components|Audio|FadeOut (Variables|Default|GetaudioComponent) 1.3 0.0 :!class /Script/Engine.AudioComponent))))

(event Custom|GameFinished
  (bind _yourapples (Variables|Default|GetyourApples))
  (bind _diglettsapplels (Variables|Default|GetdiglettsApplels))
  ;[1 1 1] Game Finished
  (bind _asdigletts_apple_gi (Utilities|Casting|CastToDiglettsAppleGI (Game|GetGameInstance)))
  (Default|FinishCurrentGame _asdigletts_apple_gi _yourapples _diglettsapplels)
  (if (not (== _yourapples _diglettsapplels))
    (if (> _yourapples _diglettsapplels)
      (Game|OpenLevel(byName) "PikachuWins")
      (elif (< _yourapples _diglettsapplels)
        (Game|OpenLevel(byName) "DiglettWins")))))

(event EventBeginPlay
  (bind _returnvalue (UserInterface|CreateWidget "/Game/UI/InGameWidget.InGameWidget_C" (Game|GetPlayerController 0)))
  (bind _output_get (Variables|Default|SetInGameWidget _returnvalue))
  (UserInterface|Viewport|AddtoPlayerScreen _output_get)
  (bind _outactors (Actor|GetAllActorsOfClass "/Game/BluePrints/Actors/AppleSpawner.AppleSpawner_C"))
  (Variables|Default|SetAppleSpawner (Utilities|Array|Get(acopy) _outactors))
  (bind _returnvalue_2 (AddComponent|AddAudioComponent false))
  (bind _output_get_2 (Variables|Default|SetaudioComponent _returnvalue_2))
  (bind _asdigletts_apple_gi (Utilities|Casting|CastToDiglettsAppleGI (Game|GetGameInstance))
    (:then
      (Audio|Components|Audio|AdjustVolume _output_get_2 0.0 (Variables|/Game/BluePrints/GameObjects/DiglettsAppleGI.DiglettsAppleGI_C|GetmusicVol _asdigletts_apple_gi) :!class /Script/Engine.AudioComponent))
    (:CastFailed
      _))
  (Audio|Components|Audio|SetSound _output_get_2 (Variables|Default|GetbgMusic))
  (Audio|Components|Audio|Play _output_get_2 0.0))

(event EventTick
  (params (DeltaSeconds :type Float%20%28single-precision%29)))

(fn ConstructionScript)

(fn GetYourApples
  (return (Variables|Default|GetyourApples)))

(fn GetDiglettsApples
  (return (Variables|Default|GetdiglettsApplels)))

(fn GetSecondsLeft
  (return (Variables|Default|GetsecLeft)))