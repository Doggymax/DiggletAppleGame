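; DiglettsAppleGI, apparently the game instance for a Digletts apple game, keeps the latest scores and level progression.
; FinishCurrentGame stores the player and Diglett scores through setters, with getters to read them back.
; A CurrentLevel index into the Levels array drives opening the current or next level by name, the latter advancing the index without a bounds check.
; Each open call passes through a DoOnce that resets right after the load call.
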(fn SetPlayerScore
  (params (thisScore :type Integer))
  (Variables|Default|SetlatestPlayerScore thisScore))

(fn SetDiglettScore
  (params (thisScore :type Integer))
  (Variables|Default|SetlatestDigletScore thisScore))

(fn FinishCurrentGame
  (params (playerScore :type Integer) (DigletScore :type Integer))
  (CallFunction|SetPlayerScore playerScore)
  (CallFunction|SetDiglettScore DigletScore))

(fn NextLevel
  (Variables|Default|SetcurrentLevel (+ (Variables|Default|GetcurrentLevel) 1)))

(fn GetPlayerLatest
  (return (Variables|Default|GetlatestPlayerScore)))

(fn GetDiglettsLatest
  (return (Variables|Default|GetlatestDigletScore)))

(fn GetCurrentLevel
  (return (Utilities|Array|Get(acopy) (Variables|Default|Getlevels) (Variables|Default|GetcurrentLevel))))

(fn OpenNextLevel
  (Utilities|FlowControl|DoOnce false :!label _label
    (:Completed
      (Game|OpenLevel(byName) (Utilities|Array|Get(acopy) (Variables|Default|Getlevels) (+ (Variables|Default|GetcurrentLevel) 1)))
      (Variables|Default|SetcurrentLevel (+ (Variables|Default|GetcurrentLevel) 1))
      (goto _label Reset))))

(fn OpenCurrentLevel
  (Utilities|FlowControl|DoOnce false :!label _label
    (:Completed
      (Game|OpenLevel(byName) (Utilities|Array|Get(acopy) (Variables|Default|Getlevels) (Variables|Default|GetcurrentLevel)))
      (goto _label Reset))))