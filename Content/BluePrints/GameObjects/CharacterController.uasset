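; Player controller that drives a PikachuBP pawn along one movement axis and handles pausing.
; BeginPlay switches the view to the first CameraActor found and caches the pawn.
; An input axis feeds forward movement, while held touches steer each Tick by comparing latest X to MiddleScreen, whose viewport-based calculation is disconnected.
; The pause action shows a reusable PauseMenuWD with UI-only input and pauses the game.
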(event EventBeginPlay
  (bind _outactors (Actor|GetAllActorsOfClass "/Script/Engine.CameraActor"))
  (if (> (Utilities|Array|Length _outactors) 0)
    (Game|Player|SetViewTargetwithBlend (Utilities|Array|Get(acopy) _outactors) 0.0 "VTBlend_Linear" 0.0 false)
    (bind _aspikachu_bp (Utilities|Casting|CastToPikachuBP (Pawn|GetControlledPawn (Game|GetPlayerController 0))))
    (Variables|Default|SetCharacterControlled _aspikachu_bp)
    (else
      (Development|PrintString "ERROR!!!" true true "(R=1.000000,G=0.000000,B=0.000000,A=1.000000)"))))

(event EventTick
  (params (DeltaSeconds :type Float%20%28single-precision%29))
  (bind _charactercontrolled (Variables|Default|GetCharacterControlled))
  (if (> (Variables|Default|GetfingersDown) 0.0)
    (if (> (Variables|Default|GetlatestPosition) (Variables|Default|GetmiddleScreen))
      (Default|AddForwardMovement _charactercontrolled -1.0)
      (else
        (Default|AddForwardMovement _charactercontrolled 1.0)))))

(event Input|ActionEvents|InputActionPauseButton
  (params (Key :type Key%20Structure))
  (:Pressed
    (Utilities|IsValid (Variables|Default|GetPauseMenuWD)
      (:Is%20Valid
        _)
      (:Is%20Not%20Valid
        (bind _returnvalue (UserInterface|CreateWidget "/Game/UI/PauseMenuWD.PauseMenuWD_C"))
        (Variables|Default|SetPauseMenuWD _returnvalue)))
    (UserInterface|Viewport|AddtoPlayerScreen (Variables|Default|GetPauseMenuWD))
    (Variables|Default|SetbShowMouseCursor true)
    (Input|SetInputModeUIOnly self (Variables|Default|GetPauseMenuWD) "DoNotLock")
    (Game|SetGamePaused true)))

(event Input|AxisEvents|InputAxisMoveForwadAxis
  (params (AxisValue :type Float%20%28single-precision%29))
  (bind _charactercontrolled (Variables|Default|GetCharacterControlled))
  (Utilities|IsValid _charactercontrolled
    (:Is%20Valid
      (Default|AddForwardMovement _charactercontrolled AxisValue))))

(event Input|TouchEvents|InputTouch
  (params (Location :type Vector) (FingerIndex :type ETouchIndex%20Enum))
  (:Pressed
    (Variables|Default|SetfingersDown (+ (Variables|Default|GetfingersDown) 1.0))
    (Variables|Default|SetlatestPosition (.X (Math|Vector|BreakVector Location)) :!label _label))
  (:Released
    (Variables|Default|SetfingersDown (- (Variables|Default|GetfingersDown) 1.0)))
  (:Moved
    (goto _label)))

(fn ConstructionScript)